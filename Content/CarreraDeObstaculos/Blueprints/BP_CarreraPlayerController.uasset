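; Player controller for the obstacle-race mode that relays race state, time, score and end-of-game messages to the player's HUD widget.
; On BeginPlay it sets game-only input, adds the default Enhanced Input context and, after a short delay, syncs the HUD with the current CarreraGameState.
; Update events cast an existing HUDInstanciado reference to WBP_HUD, with debug prints for state changes and a failed end-message cast.
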(event EventBeginPlay
  (bind _returnvalue (Class|GameplayStatics|GetPlayerControllerfromID))
  (Input|SetInputModeGameOnly _returnvalue false)
  (Input|AddMappingContext (PlayerController|LocalPlayerSubsystems|GetEnhancedInputLocalPlayerSubsystem _returnvalue) "/Game/Input/IMC_Default.IMC_Default" 0 "(bIgnoreAllPressedKeysUntilRelease=True,bForceImmediately=False,bNotifyUserSettings=False)")
  (Utilities|FlowControl|Delay 0.2)
  (bind _ascarrera_game_state (Utilities|Casting|CastToCarreraGameState (Game|GetGameState)))
  (Class|CarreraPlayerController|ActualizarEstadoHUD (Variables|/Script/CarreraDeObstaculos.CarreraGameState|GetEstadoActual _ascarrera_game_state)))

(event EventTick
  (params (DeltaSeconds :type Float%20%28single-precision%29)))

(event EventActualizarPuntajeHUD
  (params (NuevoPuntaje :type Integer))
  (bind _aswbp_hud (Utilities|Casting|CastToWBP_HUD (Variables|Default|GetHUDInstanciado)))
  (Default|ActualizarTextoPuntaje _aswbp_hud NuevoPuntaje))

(event EventMostrarFinDeJuegoHUD
  (params (Mensaje :type String))
  (bind _aswbp_hud (Utilities|Casting|CastToWBP_HUD (Variables|Default|GetHUDInstanciado))
    (:then
      (Default|MostrarMensaje _aswbp_hud (Utilities|Text|ToText(String) Mensaje)))
    (:CastFailed
      (Development|PrintString "FALLO EL CAST!!!" true true "(R=1.000000,G=0.012477,B=0.000000,A=1.000000)" 5.0))))

(event EventActualizarTiempoHUD
  (params (NuevoTiempo :type Integer))
  (bind _aswbp_hud (Utilities|Casting|CastToWBP_HUD (Variables|Default|GetHUDInstanciado)))
  (Default|ActualizarTextoTiempo _aswbp_hud NuevoTiempo))

(event EventActualizarEstadoHUD
  (params (NuevoEstado :type ECarreraEstado%20Enum :default "Esperando"))
  (Development|PrintString "ActualizaeEstadoHUD" true true "(R=1.000000,G=0.000000,B=0.990133,A=1.000000)" 5.0)
  (bind _aswbp_hud (Utilities|Casting|CastToWBP_HUD (Variables|Default|GetHUDInstanciado)))
  (switch Utilities|FlowControl|Switch|SwitchonECarreraEstado NuevoEstado
    (:Esperando
      (Default|MostrarMensaje _aswbp_hud "Esperando Jugadores")
      (Development|PrintString "EsperandoJugadores" true true "(R=0.010615,G=0.357140,B=1.000000,A=1.000000)" 5.0))
    (:Jugando
      (Default|MostrarMensaje _aswbp_hud "Inicio")
      (Development|PrintString "Largaron" true true "(R=0.000000,G=1.000000,B=0.201015,A=1.000000)" 5.0))))

(fn ConstructionScript)