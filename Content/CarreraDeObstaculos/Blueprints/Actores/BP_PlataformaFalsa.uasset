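; False platform for an obstacle race that briefly vanishes after a race character steps on it.
; On the server, the box overlap starts a DoOnce-guarded sequence that deactivates the platform after a short delay, reactivates it later, then resets.
; The replicated EstaActiva flag drives an OnRep that toggles the cube's visibility and collision on each machine.
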(event OnComponentBeginOverlap(Box)
  (params (OverlappedComponent :type Primitive%20Component%20Object%20Reference) (OtherActor :type Actor%20Object%20Reference) (OtherComp :type Primitive%20Component%20Object%20Reference) (OtherBodyIndex :type Integer) (bFromSweep :type Boolean) (SweepResult :type Hit%20Result%20Structure%20%28by%20ref%29))
  (Networking|SwitchHasAuthority
    (:Authority
      (Utilities|Casting|CastToBP_CarreraCharacter OtherActor)
      (Utilities|FlowControl|DoOnce false :!label _label
        (:Completed
          (Utilities|FlowControl|Delay 0.8)
          (Variables|Default|SetbEstaActiva? false)
          (Utilities|FlowControl|Delay 1.6)
          (Variables|Default|SetbEstaActiva? true)
          (goto _label Reset))))))

(event EventBeginPlay
  (Networking|SwitchHasAuthority
    (:Authority
      (Variables|Default|SetbEstaActiva? true))))

(event Collision|EventActorBeginOverlap
  (params (OtherActor :type Actor%20Object%20Reference)))

(event EventTick
  (params (DeltaSeconds :type Float%20%28single-precision%29)))

(fn ConstructionScript)

(fn OnRepBEstaActiva?
  (bind _cube (Variables|Default|GetCube))
  (if (Variables|Default|GetbEstaActiva?)
    (Rendering|SetVisibility _cube true false)
    (Collision|SetCollisionEnabled _cube "QueryAndPhysics")
    (else
      (Rendering|SetVisibility _cube false false)
      (Collision|SetCollisionEnabled _cube "NoCollision"))))