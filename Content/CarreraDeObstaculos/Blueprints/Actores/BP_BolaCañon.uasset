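; Cannonball actor for the obstacle race that knocks racers back when it hits them at speed and expires a few seconds after spawning.
; On the server only, a sphere component hit against a BP_CarreraCharacter checks that the ball is moving above a speed threshold.
; It then launches the character away from the ball's center with an added upward boost, overriding existing velocity.
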(event OnComponentHit(Sphere1)
  (params (HitComponent :type Primitive%20Component%20Object%20Reference) (OtherActor :type Actor%20Object%20Reference) (OtherComp :type Primitive%20Component%20Object%20Reference) (NormalImpulse :type Vector :default "0, 0, 0") (Hit :type Hit%20Result%20Structure%20%28by%20ref%29))
  (Networking|SwitchHasAuthority
    (:Authority
      (bind _asbp_carrera_character (Utilities|Casting|CastToBP_CarreraCharacter OtherActor))
      (if (> (Math|Vector|VectorLength (Transformation|GetVelocity)) 2.5e+02)
        (Character|LaunchCharacter _asbp_carrera_character (+ (* (Math|Vector|Normalize (- (Transformation|GetActorLocation _asbp_carrera_character) (Transformation|GetActorLocation))) 1.5e+03) "0.000000,0.000000,500.000000") true true)))))

(event EventBeginPlay
  (Actor|SetLifeSpan 5.0))

(event Collision|EventActorBeginOverlap
  (params (OtherActor :type Actor%20Object%20Reference)))

(event EventTick
  (params (DeltaSeconds :type Float%20%28single-precision%29)))

(fn ConstructionScript)