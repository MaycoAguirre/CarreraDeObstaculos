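; BP_Pendulo is a swinging pendulum obstacle for the obstacle race that knocks characters away.
; On the server, a timeline drives the actor's roll after a random start delay.
; Each server tick polls the ball sphere for overlapping race characters and launches them along the ball's direction of travel with an upward boost.
; That direction comes from the difference between the ball's current and previous-tick positions.
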(event EventBeginPlay
  (Networking|SwitchHasAuthority
    (:Authority
      (Utilities|FlowControl|Delay (Math|Random|RandomFloatinRange 0.0 3.0))
      (bind _rotacion (Timeline|TL_Columpio PlayFromStart)
        (:Update
          (Transformation|SetActorRotation (Math|Rotator|MakeRotator _rotacion 0.0 0.0)))))))

(event Collision|EventActorBeginOverlap
  (params (OtherActor :type Actor%20Object%20Reference)))

(event EventTick
  (params (DeltaSeconds :type Float%20%28single-precision%29))
  (bind _sphere2 (Variables|Default|GetSphere2))
  (Networking|SwitchHasAuthority
    (:Authority
      (for _array_element (Collision|GetOverlappingActors _sphere2 "/Game/CarreraDeObstaculos/Blueprints/BP_CarreraCharacter.BP_CarreraCharacter_C" :!class /Script/Engine.PrimitiveComponent)
        (bind _asbp_carrera_character (Utilities|Casting|CastToBP_CarreraCharacter _array_element))
        (Character|LaunchCharacter _asbp_carrera_character (+ (* (Math|Vector|Normalize (- (Transformation|GetWorldLocation (Variables|Default|GetSphere2)) (Variables|Default|GetPosicionAnteriorBola))) 2e+03) "0.000000,0.000000,800.000000") true true))
      (Variables|Default|SetPosicionAnteriorBola (Transformation|GetWorldLocation _sphere2)))))

(fn ConstructionScript)