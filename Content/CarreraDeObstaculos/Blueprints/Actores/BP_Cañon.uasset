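; BP_Cañon is a cannon actor for the obstacle course that repeatedly fires BP_BolaCañon balls.
; On BeginPlay, only the authority starts a looping timer, with an interval randomized once per cannon.
; Each Disparar event spawns a ball at the Arrow component's transform and launches its sphere along the arrow's forward vector with a mass-independent velocity-change impulse.
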(event Custom|Disparar
  (bind _returnvalue (Game|SpawnActorfromClass "/Game/CarreraDeObstaculos/Blueprints/Actores/BP_BolaCañon.BP_BolaCañon_C" (Transformation|GetWorldTransform (Variables|Default|GetArrow)) "Undefined" "MultiplyWithRoot" 0 0))
  (Physics|AddImpulse (Variables|/Game/CarreraDeObstaculos/Blueprints/Actores/BP_BolaCañon.BP_BolaCañon_C|GetSphere1 _returnvalue) (* (Math|Vector|GetForwardVector (Variables|Default|GetArrow)) 5e+02) "None" true))

(event EventBeginPlay
  (Networking|SwitchHasAuthority
    (:Authority
      (Utilities|Time|SetTimerbyEvent (delegate Custom|Disparar) (Math|Random|RandomFloatinRange 1.5 5.0) true))))

(event Collision|EventActorBeginOverlap
  (params (OtherActor :type Actor%20Object%20Reference)))

(event EventTick
  (params (DeltaSeconds :type Float%20%28single-precision%29)))

(fn ConstructionScript)