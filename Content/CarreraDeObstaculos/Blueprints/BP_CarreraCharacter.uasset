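; Player character for an obstacle race, handling movement, camera look, jump, grab and push through Enhanced Input events.
; Movement follows the control rotation's yaw and applies only while CarreraGameState reports PuedeMoverse; look, jump, grab and push have no such check here.
; Grab and push call IntentarAgarrar and IntentarEmpujar, whose logic lives outside these graphs.
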(event Input|EnhancedActionEvents|EnhancedInputActionIA_Agarrar
  (params (ActionValue :type Boolean) (ElapsedSeconds :type Float%20%28double-precision%29) (TriggeredSeconds :type Float%20%28double-precision%29) (InputAction :type Input%20Action%20Object%20Reference :default "/Game/Input/Actions/IA_Agarrar.IA_Agarrar"))
  ;[0.15 0 0.001287 0.5] Inputs
  (:Started
    (Class|CarreraDeObstaculosCharacter|IntentarAgarrar)))

(event Input|EnhancedActionEvents|EnhancedInputActionIA_MouseLook
  (params (ActionValue :type Vector%202D%20Structure) (ElapsedSeconds :type Float%20%28double-precision%29) (TriggeredSeconds :type Float%20%28double-precision%29) (InputAction :type Input%20Action%20Object%20Reference :default "/Game/Input/Actions/IA_MouseLook.IA_MouseLook"))
  ;[0.15 0 0.001287 0.5] Inputs
  (Pawn|Input|AddControllerYawInput (.x ActionValue))
  (Pawn|Input|AddControllerPitchInput (.y ActionValue)))

(event Input|EnhancedActionEvents|EnhancedInputActionIA_Move
  (params (ActionValue :type Vector%202D%20Structure) (ElapsedSeconds :type Float%20%28double-precision%29) (TriggeredSeconds :type Float%20%28double-precision%29) (InputAction :type Input%20Action%20Object%20Reference :default "/Game/Input/Actions/IA_Move.IA_Move"))
  (bind _returnvalue (Pawn|GetControlRotation :!class /Script/Engine.Pawn))
  (bind _returnvalue_2 (Math|Rotator|MakeRotator 0.0 0.0 (.yaw _returnvalue)))
  ;[0.15 0 0.001287 0.5] Inputs
  (bind _ascarrera_game_state (Utilities|Casting|CastToCarreraGameState (Game|GetGameState)))
  (if (Class|CarreraGameState|PuedeMoverse _ascarrera_game_state)
    (Pawn|Input|AddMovementInput (Math|Vector|GetForwardVector _returnvalue_2) (.y ActionValue) false)
    (Pawn|Input|AddMovementInput (Math|Vector|GetRightVector _returnvalue_2) (.x ActionValue) false)))

(event Input|EnhancedActionEvents|EnhancedInputActionIA_Jump
  (params (ActionValue :type Boolean) (ElapsedSeconds :type Float%20%28double-precision%29) (TriggeredSeconds :type Float%20%28double-precision%29) (InputAction :type Input%20Action%20Object%20Reference :default "/Game/Input/Actions/IA_Jump.IA_Jump"))
  ;[0.15 0 0.001287 0.5] Inputs
  (:Started
    (Character|Jump)))

(event Input|EnhancedActionEvents|EnhancedInputActionIA_Empujar
  (params (ActionValue :type Boolean) (ElapsedSeconds :type Float%20%28double-precision%29) (TriggeredSeconds :type Float%20%28double-precision%29) (InputAction :type Input%20Action%20Object%20Reference :default "/Game/Input/Actions/IA_Empujar.IA_Empujar"))
  ;[0.15 0 0.001287 0.5] Inputs
  (:Started
    (Class|CarreraDeObstaculosCharacter|IntentarEmpujar)))

(event EventBeginPlay)

(event Collision|EventActorBeginOverlap
  (params (OtherActor :type Actor%20Object%20Reference)))

(event EventTick
  (params (DeltaSeconds :type Float%20%28single-precision%29)))

(fn ConstructionScript)